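; BP_FieldSystem is a field system Blueprint that applies a disable-threshold physics field over a box volume when play begins.
; A box falloff with a fixed magnitude supplies the threshold value, and a culling field built from a second box falloff culls it outside the volume.
; Both boxes take the FieldSystemComponent's world transform and use no falloff, so the actor's placement defines the affected region.
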(event `self.ReceiveBeginPlay`
  (bind _returnvalue (`SceneComponent.K2_GetComponentToWorld` (`self.FieldSystemComponent`)))
  (`FieldSystemComponent.ApplyPhysicsField` (`self.FieldSystemComponent`) true "Field_DisableThreshold" null (`CullingField.SetCullingField` (`self.CullingField`) (`BoxFalloff.SetBoxFalloff` (`self.BoxFalloffMagnitude`) 1.0 0.0 1.0 0.0 _returnvalue "Field_FallOff_None") (`BoxFalloff.SetBoxFalloff` (`self.BoxFalloff`) 1001.0 (`self.Falloff Max X`) (`self.Falloff Max Y`) 0.0 _returnvalue "Field_FallOff_None") "Field_Culling_Outside")))

(fn `UserConstructionScript`)